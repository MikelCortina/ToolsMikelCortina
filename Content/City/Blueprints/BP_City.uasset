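; BP_City is a procedural city actor that drives a PCG component to build a city from size, block and building parameters.
; Generate sizes the bounds box, pushes the parameters into the graph instance, sets the seed and runs local generation.
; Cleanup clears PCG output and destroys all actors tagged CityGenerated.
; Snapshot stores the instance count and a weighted location-and-scale checksum of its instanced meshes as a signature string for comparing results.
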(event EventBeginPlay)

(event Collision|EventActorBeginOverlap
  (params (OtherActor :type Actor%20Object%20Reference)))

(event EventTick
  (params (DeltaSeconds :type Float%20%28single-precision%29)))

(fn ConstructionScript)

(fn Generate
  (bind _citysize (Variables|Ciudad|GetCitySize))
  (bind _pcg (Variables|Default|GetPCG))
  (bind _returnvalue (* _citysize 5e+01))
  (bind _graphinstance (Variables|/Script/PCG.PCGComponent|GetGraphInstance _pcg))
  (Components|Box|SetBoxExtent (Variables|Default|GetCityBounds) (Math|Vector|MakeVector _returnvalue _returnvalue 5e+02) true)
  (Class|PCGGraphParametersHelpers|SetDoubleParameter _graphinstance "CitySize" (Variables|Ciudad|GetCitySize))
  (Class|PCGGraphParametersHelpers|SetDoubleParameter _graphinstance "BlockSize" (Variables|Ciudad|GetBlockSize))
  (Class|PCGGraphParametersHelpers|SetDoubleParameter _graphinstance "BuildingDensity" (Variables|Ciudad|GetBuildingDensity))
  (Class|PCGGraphParametersHelpers|SetDoubleParameter _graphinstance "BuildingHeight" (Variables|Ciudad|GetBuildingHeight))
  (Class|PCGGraphParametersHelpers|SetDoubleParameter _graphinstance "BuildingVariation" (Variables|Ciudad|GetBuildingVariation))
  (Variables|/Script/PCG.PCGComponent|SetSeed _pcg (Variables|Ciudad|GetSeed))
  (Class|PCGComponent|GenerateLocal _pcg true))

(fn Cleanup
  (Class|PCGComponent|CleanupLocal (Variables|Default|GetPCG) true)
  (bind _outactors (Actor|GetAllActorswithTag "CityGenerated"))
  (for _array_element _outactors
    (Actor|DestroyActor _array_element)))

(fn Snapshot
  (Variables|Ciudad|Test|SetSnapCount 0)
  (Variables|Ciudad|Test|SetSnapSum 0.0)
  (for _array_element (Actor|GetComponentsByClass "/Script/Engine.InstancedStaticMeshComponent")
    (bind _asinstanced_static_mesh_component (Utilities|Casting|CastToInstancedStaticMeshComponent _array_element))
    (for _index (range 0 (- (Components|InstancedStaticMesh|GetInstanceCount _asinstanced_static_mesh_component) 1))
      (Variables|Ciudad|Test|SetSnapSum (+ (+ (Math|Vector|DotProduct (.Location (Math|Transform|BreakTransform (.OutInstanceTransform (Components|InstancedStaticMesh|GetInstanceTransform _asinstanced_static_mesh_component _index true)))) "1.0,2.0,3.0") (Math|Vector|DotProduct (.Scale (Math|Transform|BreakTransform (.OutInstanceTransform (Components|InstancedStaticMesh|GetInstanceTransform _asinstanced_static_mesh_component _index true)))) "1000.0,2000.0,3000.0")) (Variables|Ciudad|Test|GetSnapSum)))
      (Variables|Ciudad|Test|SetSnapCount (+ (Variables|Ciudad|Test|GetSnapCount) 1))))
  (Variables|Ciudad|Test|SetLastSnapshot (Utilities|String|Append (Utilities|String|Append (Utilities|String|ToString(Integer) (Variables|Ciudad|Test|GetSnapCount)) " instancias / firma ") (Utilities|String|ToString(Float) (Variables|Ciudad|Test|GetSnapSum)))))